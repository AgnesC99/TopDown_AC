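; BP_SplinePatrol is a patrolling enemy that moves along a spline and detects the player through a trigger.
; Each Tick advances a distance along the spline at constant speed, moving a sphere to that point and looping back to the start at the end.
; Player overlap turns the spotlight red, prints a death message and zeroes the distance, freezing the sphere in place.
; Ending overlap restores grey light and resumes patrol from the spline's start.
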(event OnComponentBeginOverlap(Trigger)
  (params (OverlappedComponent :type Primitive%20Component%20Object%20Reference) (OtherActor :type Actor%20Object%20Reference) (OtherComp :type Primitive%20Component%20Object%20Reference) (OtherBodyIndex :type Integer) (bFromSweep :type Boolean) (SweepResult :type Hit%20Result%20Structure%20%28by%20ref%29))
  ;[1 1 1] Identifying player
  (Utilities|Casting|CastToCore_PlayerCharacter OtherActor)
  (Development|PrintString "YOU ARE DEAD" true true "(R=1.000000,G=0.000000,B=0.020607,A=1.000000)")
  (Rendering|Components|Light|SetLightColor (Variables|Default|GetSpotLight) "(R=1.000000,G=0.000000,B=0.008568,A=1.000000)" true)
  (Variables|Default|SetbIfDetected true))

(event OnComponentEndOverlap(Trigger)
  (params (OverlappedComponent :type Primitive%20Component%20Object%20Reference) (OtherActor :type Actor%20Object%20Reference) (OtherComp :type Primitive%20Component%20Object%20Reference) (OtherBodyIndex :type Integer))
  ;[1 1 1] Identifying player
  (Utilities|Casting|CastToCore_PlayerCharacter OtherActor)
  (Development|PrintString "Where did you go?" true true "(R=1.000000,G=0.449096,B=0.000000,A=1.000000)")
  (Rendering|Components|Light|SetLightColor (Variables|Default|GetSpotLight) "(R=0.093059,G=0.093059,B=0.093059,A=1.000000)" true)
  (Variables|Default|SetbIfDetected false))

(event EventTick
  (params (DeltaSeconds :type Float%20%28single-precision%29))
  (bind _spline (Variables|Default|GetSpline))
  (bind _returnvalue (Spline|GetSplineLength _spline))
  ;[1 1 1] Travelling on spline
  (if (Variables|Default|GetbIfDetected)
    (Variables|Default|SetCurrentDistanceAlongSpline 0.0)
    (elif (>= (Variables|Default|GetCurrentDistanceAlongSpline) _returnvalue)
      (Variables|Default|SetCurrentDistanceAlongSpline 0.0)
      (else
        (bind _output_get (Variables|Default|SetCurrentDistanceAlongSpline (Math|Interpolation|FInterptoConstant (Variables|Default|GetCurrentDistanceAlongSpline) _returnvalue DeltaSeconds (Variables|Default|GetEnemyTravellingSpeed))))
        (Transformation|SetRelativeLocation (Variables|Default|GetSphere) (Spline|GetLocationatDistanceAlongSpline (Variables|Default|GetSpline) _output_get "Local") false false)))))

(fn ConstructionScript)